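; VR Morse telegraph interactable that turns button presses into letters and prints the word built so far.
; Holding the VR button plays a sound while Tick times it; on release, DotOrDash stores whichever is nearer, one or three TimeUnits.
; After seven idle units, GetMorseLetter decodes the buffer through a branch tree and appends to CurrentWord.
; The two-symbol branch tests the first symbol twice, so A and N are unreachable.
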(event `self.ReceiveBeginPlay`
  (bind _returnvalue (`GameplayStatics.SpawnSoundAtLocation` (`self.Sound`) (`SceneComponent.K2_GetComponentLocation` (`self.VRButton`)) (struct) 1.0 1.0 0.0 null null))
  (set `self.CurrentSound` _returnvalue)
  (`AudioComponent.SetPaused` (`self.CurrentSound`) true))

(event `self.VRButton.OnButtonStateChanged`
  (params (ButtonState :type Boolean) (InteractingActor :type "Actor Object Reference") (InteractingComponent :type "PrimitiveComponent Object Reference"))
  (bind _output_get (set `self.IsButtonDown` ButtonState))
  (if _output_get
    (set `self.TimeSinceLastDown` 0.0)
    (`AudioComponent.SetPaused` (`self.CurrentSound`) false)
    (else
      (bind _true___dot (`self.DotOrDash` (`self.HeldDownForSeconds`)))
      (`KismetArrayLibrary.Array_Add` (`self.EnteredMorse`) _true___dot)
      (set `self.HeldDownForSeconds` 0.0)
      (`AudioComponent.SetPaused` (`self.CurrentSound`) true))))

(event `self.ReceiveTick`
  (params (DeltaSeconds :type "Float (single-precision)"))
  (if (`self.IsButtonDown`)
    (set `self.HeldDownForSeconds` (+ (`self.HeldDownForSeconds`) DeltaSeconds))
    (else
      (bind _output_get (set `self.TimeSinceLastDown` (+ (`self.TimeSinceLastDown`) DeltaSeconds)))
      (if (and (>= _output_get (* (`self.TimeUnit`) 7.0)) (> (`KismetArrayLibrary.Array_Length` (`self.EnteredMorse`)) 0))
        (bind _letter (`self.GetMorseLetter`))
        (bind _output_get_2 (set `self.CurrentWord` (`KismetStringLibrary.Concat_StrStr` (`self.CurrentWord`) _letter)))
        (`KismetSystemLibrary.PrintString` _output_get_2 true true (struct :`G` 0.66 :`B` 1.0 :`A` 1.0) 200.0)
        (`KismetArrayLibrary.Array_Clear` (`self.EnteredMorse`))))))

(fn `DotOrDash`
  (params (HeldDownFor :type "Float (double-precision)"))
  (returns (`True = Dot` :type Boolean))
  (bind _timeunit (`self.TimeUnit`))
  (return (< (`KismetMathLibrary.Abs` (- HeldDownFor _timeunit)) (`KismetMathLibrary.Abs` (- HeldDownFor (* _timeunit 3.0))))))

(fn `GetMorseLetter`
  (returns (Letter :type String))
  (bind _output (`|GetArrayItem` (`self.EnteredMorse`) 1))
  (bind _output_2 (`|GetArrayItem` (`self.EnteredMorse`) 2))
  (bind _output_3 (`|GetArrayItem` (`self.EnteredMorse`) 3))
  (bind _output_4 (`|GetArrayItem` (`self.EnteredMorse`)))
  (bind _output_5 (`|GetArrayItem` (`self.EnteredMorse`) 1))
  (bind _output_6 (`|GetArrayItem` (`self.EnteredMorse`) 2))
  (switch `int` (`KismetArrayLibrary.Array_Length` (`self.EnteredMorse`))
    (:`1`
      (if (`|GetArrayItem` (`self.EnteredMorse`))
        (return "E")
        (else
          (return "T"))))
    (:`2`
      (if (`|GetArrayItem` (`self.EnteredMorse`))
        (if _output_4
          (return "I")
          (else
            (return "A")))
        (elif _output_4
          (return "N")
          (else
            (return "M")))))
    (:`3`
      (if (`|GetArrayItem` (`self.EnteredMorse`))
        (if _output
          (if _output_2
            (return "S")
            (else
              (return "U")))
          (elif _output_2
            (return "R")
            (else
              (return "W"))))
        (elif _output
          (if _output_2
            (return "D")
            (else
              (return "K")))
          (elif _output_2
            (return "G")
            (else
              (return "O"))))))
    (:`4`
      (if (`|GetArrayItem` (`self.EnteredMorse`))
        (if _output_5
          (if _output_6
            (if _output_3
              (return "H")
              (else
                (return "V")))
            (elif _output_3
              (return "F")
              (else
                (return "Invalid"))))
          (elif _output_6
            (if _output_3
              (return "L")
              (else
                (return "Invalid")))
            (elif _output_3
              (return "P")
              (else
                (return "J")))))
        (elif _output_5
          (if _output_6
            (if _output_3
              (return "B")
              (else
                (return "X")))
            (elif _output_3
              (return "C")
              (else
                (return "Y"))))
          (elif _output_6
            (if _output_3
              (return "Z")
              (else
                (return "Q")))
            (else
              (return "Invalid"))))))))

(fn `ResetWord`
  (set `self.CurrentWord` ""))

(fn `UserConstructionScript`)