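; BP_LightSwitch is a VR button switch that lets the player toggle the level's lights.
; At BeginPlay it caches the level's BP_LightDarkManager.
; When the VRButton changes to the pressed state through BP_Player's left or right trigger component, it plays a placeholder switch sound and calls ToggleLights on the manager.
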(event `self.ReceiveBeginPlay`
  (bind _returnvalue (`GameplayStatics.GetActorOfClass` "/Game/Blueprints/Light-Dark_System/BP_LightDarkManager.BP_LightDarkManager_C"))
  (set `self.LightDarkRef` _returnvalue))

(event `self.VRButton.OnButtonStateChanged`
  (params (ButtonState :type Boolean) (InteractingActor :type "Actor Object Reference") (InteractingComponent :type "PrimitiveComponent Object Reference"))
  (bind _asbp_player (cast `/Game/Blueprints/Player/BP_Player` InteractingActor))
  (if (== (`/Game/Blueprints/Player/BP_Player.Left Trigger` _asbp_player) InteractingComponent)
    (if ButtonState :!label _label
      (`AudioComponent.Play` (`self.A_PLACEHOLDER_LightSwitch_Cue`) 0.0)
      (`/Game/Blueprints/Light-Dark_System/BP_LightDarkManager.ToggleLights` (`self.LightDarkRef`)))
    (elif (== (`/Game/Blueprints/Player/BP_Player.Right Trigger` _asbp_player) InteractingComponent)
      (goto _label))))

(fn `UserConstructionScript`)