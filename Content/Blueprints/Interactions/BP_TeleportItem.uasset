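; BP_TeleportItem is a grippable cube that moves the game from the Introduction section to the FirstEncounter section by swapping streamed levels.
; On the first grip, a Teleported flag blocks repeats and a sequence unloads the Introduction blockout, content and lighting levels without blocking.
; It then loads the FirstEncounter equivalents plus a doorway level with blocking loads, making them visible.
; An older player teleport by a fixed offset remains disconnected and never runs.
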(event `self.Cube.OnGripped`
  (params (GrippingController :type "GripMotionControllerComponent Object Reference") (GripInformation :type "BPActorGripInformation Structure (by ref)"))
  (if (not (`self.Teleported`))
    (set `self.Teleported` true)
    (`|ExecutionSequence`
      (:`then_0`
        (`GameplayStatics.UnloadStreamLevelBySoftObjectPtr` "/Game/Levels/Demo/Introduction/L_Introduction_Blockout.L_Introduction_Blockout"))
      (:`then_1`
        (`GameplayStatics.UnloadStreamLevelBySoftObjectPtr` "/Game/Levels/Demo/Introduction/L_Introduction_Content.L_Introduction_Content"))
      (:`then_2`
        (`GameplayStatics.UnloadStreamLevelBySoftObjectPtr` "/Game/Levels/Demo/Introduction/L_Introduction_Lighting.L_Introduction_Lighting"))
      (:`then_3`
        (`GameplayStatics.LoadStreamLevelBySoftObjectPtr` "/Game/Levels/Demo/EnemyFIrstEncounter/L_FirstEncounter_Blockout.L_FirstEncounter_Blockout" true true))
      (:`then_4`
        (`GameplayStatics.LoadStreamLevelBySoftObjectPtr` "/Game/Levels/Demo/EnemyFIrstEncounter/L_FirstEncounter_Content.L_FirstEncounter_Content" true true))
      (:`then_5`
        (`GameplayStatics.LoadStreamLevelBySoftObjectPtr` "/Game/Levels/Demo/EnemyFIrstEncounter/L_FirstEncounter_Lighting.L_FirstEncounter_Lighting" true true))
      (:`then_6`
        (`GameplayStatics.LoadStreamLevelBySoftObjectPtr` "/Game/Levels/Demo/EnemyFIrstEncounter/L_FirstEncounter_Doorway.L_FirstEncounter_Doorway" true true)))))

(fn `UserConstructionScript`)