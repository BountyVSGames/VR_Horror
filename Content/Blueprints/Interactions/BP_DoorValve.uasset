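; BP_DoorValve is a VR door with a valve, which plays a metal slam and opens the door when its interaction completes.
; The door is set up on BeginPlay, where the squeak sound's finished callback is also bound.
; Tick compares valve and door rotations against buffered values and plays a squeak while either moves, lower pitched for the door.
; A shared IsPlaying flag prevents retriggering until the squeak finishes.
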(event `self.VRValve.OnDialFinishedLerping`)

(event `InteractionInterface.InteractionCompleted`
  (`AudioComponent.Play` (`self.A_MetalSlam_Cue`) 0.0)
  (`VRDoorComponent.OpenDoor` (`self.VRDoor`)))

(event `self.ReceiveBeginPlay`
  (`VRDoorComponent.SetupDoor` (`self.VRDoor`))
  (add `AudioComponent.OnAudioFinished` (`self.A_MetalSqueak`) (delegate `OnAudioFinished_Event`))
  (set `self.rotationBuffer` (`SceneComponent.RelativeRotation` (`self.VRValve`))))

(event `OnAudioFinished_Event`
  (set `self.IsPlaying` false))

(event `self.ReceiveTick`
  (params (DeltaSeconds :type "Float (single-precision)"))
  (bind _a_metalsqueak (`self.A_MetalSqueak`))
  (bind _a_metalsqueak_2 (`self.A_MetalSqueak`))
  (bind _relativerotation (`SceneComponent.RelativeRotation` (`self.VRDoor`)))
  (bind _relativerotation_2 (`SceneComponent.RelativeRotation` (`self.VRValve`)))
  (`|ExecutionSequence`
    (:`then_0`
      (if (!= _relativerotation_2 (`self.rotationBuffer`))
        (if (not (`self.IsPlaying`))
          (set `self.IsPlaying` true)
          (set `AudioComponent.PitchMultiplier` 1.0 _a_metalsqueak)
          (`AudioComponent.Play` _a_metalsqueak 0.0)))
      (set `self.rotationBuffer` _relativerotation_2))
    (:`then_1`
      (if (!= _relativerotation (`self.DoorRotationBuffer`))
        (if (not (`self.IsPlaying`))
          (set `self.IsPlaying` true)
          (set `AudioComponent.PitchMultiplier` 0.8 _a_metalsqueak_2)
          (`AudioComponent.Play` _a_metalsqueak_2 0.0)))
      (set `self.DoorRotationBuffer` _relativerotation))))

(fn `UserConstructionScript`)