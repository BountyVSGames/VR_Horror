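; Trigger volume that moves a referenced enemy's patrol to another spline when the player enters its box.
; On overlap, it always assigns the referenced spline as the enemy's patrol path.
; If the enemy does not have the player in sight, it first teleports the enemy to just above that spline actor's root, so the relocation is skipped while the player is spotted.
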(event `self.Box.OnComponentBeginOverlap`
  (params (OverlappedComponent :type "PrimitiveComponent Object Reference") (OtherActor :type "Actor Object Reference") (OtherComp :type "PrimitiveComponent Object Reference") (OtherBodyIndex :type Integer) (bFromSweep :type Boolean) (SweepResult :type "HitResult Structure (by ref)"))
  (bind (_returnvalue_x _returnvalue_y _returnvalue_z) (`KismetMathLibrary.BreakVector` (`SceneComponent.K2_GetComponentLocation` (`/Game/Blueprints/Enemy/Blueprint/BP_PatrolSpline.DefaultSceneRoot` (`self.Spline Reference`)))))
  (cast `/Game/Blueprints/Player/BP_Player` OtherActor)
  (if (`/Game/Blueprints/Enemy/BP_Enemy.PlayerInSight` (`self.Enemy Reference`))
    (set `/Game/Blueprints/Enemy/BP_Enemy.Patrol Spline` (`self.Spline Reference`) (`self.Enemy Reference`))
    (else
      (`self.K2_TeleportTo` :`self` (`self.Enemy Reference`) :`DestLocation` (`KismetMathLibrary.MakeVector` _returnvalue_x _returnvalue_y (+ _returnvalue_z 88.0)))
      (set `/Game/Blueprints/Enemy/BP_Enemy.Patrol Spline` (`self.Spline Reference`) (`self.Enemy Reference`)))))

(fn `UserConstructionScript`)