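; Lamp socket in the key-lock interaction system that accepts a light bulb and reveals the next puzzle elements.
; When an actor with the desired tag overlaps the sphere and casts to BP_LightBulb, it simulates a drop, destroys the bulb and turns up the point light.
; It then unhides and enables the VR button on every BP_LightSwitch and shows the first text actor tagged "Letter".
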(event `self.Sphere.OnComponentBeginOverlap`
  (params (OverlappedComponent :type "PrimitiveComponent Object Reference") (OtherActor :type "Actor Object Reference") (OtherComp :type "PrimitiveComponent Object Reference") (OtherBodyIndex :type Integer) (bFromSweep :type Boolean) (SweepResult :type "HitResult Structure (by ref)"))
  (if (`self.ActorHasTag` OtherActor (`self.Desired Tag`))
    (bind _asbp_light_bulb (cast `/Game/Blueprints/Interactions/KeyLockSystem/BP_LightBulb` OtherActor))
    (message `VRGripInterface.SimulateOnDrop` _asbp_light_bulb)
    (`self.K2_DestroyActor` _asbp_light_bulb)
    (`LightComponent.SetIntensity` (`self.PointLight`) 500.0)
    (bind _outactors (`GameplayStatics.GetAllActorsOfClass` "/Game/Blueprints/Interactions/BP_LightSwitch.BP_LightSwitch_C"))
    (for _array_element _outactors
      (bind _vrbutton (`/Game/Blueprints/Interactions/BP_LightSwitch.VRButton` _array_element))
      (`SceneComponent.SetHiddenInGame` _vrbutton false false)
      (`SceneComponent.SetHiddenInGame` (`/Game/Blueprints/Interactions/BP_LightSwitch.Cube` _array_element) false false)
      (set `VRButtonComponent.bIsEnabled` true _vrbutton))
    (bind _outactors_2 (`GameplayStatics.GetAllActorsOfClass` "/Script/Engine.TextRenderActor"))
    (for _array_element_2 _outactors_2
      (if (`self.ActorHasTag` _array_element_2 "Letter")
        (set `self.Array Element_0` _array_element_2)
        (break)))
    (`SceneComponent.SetVisibility` (`TextRenderActor.TextRender` (`self.Array Element_0`)) true false)))

(fn `UserConstructionScript`
  (`parent.UserConstructionScript`))