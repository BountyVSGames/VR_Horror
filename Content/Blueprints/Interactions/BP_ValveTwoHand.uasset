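; BP_ValveTwoHand is a VR valve interaction Blueprint that plays a metal squeak sound while the valve rotates.
; Tick compares the valve's relative rotation with the value buffered from the previous frame and starts the audio on any change.
; An IsPlaying flag prevents restarts until OnAudioFinished clears it, so the squeak plays to completion because the stop logic is disconnected.
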(event `self.ReceiveBeginPlay`
  (add `AudioComponent.OnAudioFinished` (`self.A_MetalSqueak`) (delegate `OnAudioFinished_Event`))
  (set `self.rotationBuffer` (`SceneComponent.RelativeRotation` (`self.VRValve`))))

(event `OnAudioFinished_Event`
  (set `self.IsPlaying` false))

(event `self.ReceiveTick`
  (params (DeltaSeconds :type "Float (single-precision)"))
  (bind _relativerotation (`SceneComponent.RelativeRotation` (`self.VRValve`)))
  (if (!= _relativerotation (`self.rotationBuffer`))
    (if (not (`self.IsPlaying`))
      (set `self.IsPlaying` true)
      (`AudioComponent.Play` (`self.A_MetalSqueak`) 0.0)))
  (set `self.rotationBuffer` _relativerotation))

(fn `UserConstructionScript`)