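; Steam hazard actor that uses two steam effects and two blocking volumes to block or clear an area.
; BeginPlay sets both effects and the volumes' collision from IsActive.
; InteractionCompleted applies the opposite state but never updates IsActive, so repeat interactions do not toggle it back.
; Every branch stops the SteamHiss audio, and none starts it.
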(event `self.ReceiveBeginPlay`
  (if (`self.IsActive?`)
    (`ActorComponent.SetActive` (`self.Steam_1`) true false)
    (`ActorComponent.SetActive` (`self.Steam_2`) true false)
    (`PrimitiveComponent.SetCollisionEnabled` (`self.BlockingVolume_1`) "QueryAndPhysics")
    (`PrimitiveComponent.SetCollisionEnabled` (`self.BlockingVolume_2`) "QueryAndPhysics")
    (`AudioComponent.Stop` (`self.SteamHiss`))
    (else
      (`ActorComponent.SetActive` (`self.Steam_1`) false false)
      (`ActorComponent.SetActive` (`self.Steam_2`) false false)
      (`PrimitiveComponent.SetCollisionEnabled` (`self.BlockingVolume_1`) "NoCollision")
      (`PrimitiveComponent.SetCollisionEnabled` (`self.BlockingVolume_2`) "NoCollision")
      (`AudioComponent.Stop` (`self.SteamHiss`)))))

(event `InteractionInterface.InteractionCompleted`
  (if (`self.IsActive?`)
    (`ActorComponent.SetActive` (`self.Steam_1`) false false)
    (`ActorComponent.SetActive` (`self.Steam_2`) false false)
    (`PrimitiveComponent.SetCollisionEnabled` (`self.BlockingVolume_1`) "NoCollision")
    (`PrimitiveComponent.SetCollisionEnabled` (`self.BlockingVolume_2`) "NoCollision")
    (`AudioComponent.Stop` (`self.SteamHiss`))
    (else
      (`ActorComponent.SetActive` (`self.Steam_1`) true false)
      (`ActorComponent.SetActive` (`self.Steam_2`) true false)
      (`PrimitiveComponent.SetCollisionEnabled` (`self.BlockingVolume_1`) "QueryAndPhysics")
      (`PrimitiveComponent.SetCollisionEnabled` (`self.BlockingVolume_2`) "QueryAndPhysics")
      (`AudioComponent.Stop` (`self.SteamHiss`)))))

(fn `UserConstructionScript`)