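; BP_AmbienceClang is an actor that plays an ambient metal clang sound.
; Its PlaySoundEvent randomly picks between a deep metal clang cue and a regular one and plays it from the start.
; BeginPlay, overlap and Tick are disabled stubs, so nothing in the file triggers the sound itself.
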(event `self.PlaySoundEvent`
  (`AudioComponent.Play` (select `bool` (`KismetMathLibrary.RandomBool`) :`false` (`self.A_MetalClang_Cue`) :`true` (`self.A_DeepMetalClang_Cue`)) 0.0))

(fn `UserConstructionScript`
  (`parent.UserConstructionScript`))