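; BP_ThrowableTrue is a throwable prop that makes an AI-audible noise when it hits something while not held.
; When its Sphere begins overlapping anything other than the player, it checks that the GrippableStaticMesh is not gripped.
; It then reports a noise event at the mesh's location with the player as instigator, and plays a metal clang there.
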(event `self.Sphere.OnComponentBeginOverlap`
  (params (OverlappedComponent :type "PrimitiveComponent Object Reference") (OtherActor :type "Actor Object Reference") (OtherComp :type "PrimitiveComponent Object Reference") (OtherBodyIndex :type Integer) (bFromSweep :type Boolean) (SweepResult :type "HitResult Structure (by ref)"))
  (bind _returnvalue (`GameplayStatics.GetPlayerCharacter` 0))
  (bind _returnvalue_2 (`SceneComponent.K2_GetComponentLocation` (`self.GrippableStaticMesh`)))
  (bind (_holdingcontrollers _bisheld) (`VRGripInterface.IsHeld` (`self.GrippableStaticMesh`)))
  (if _bisheld
    _
    (elif (!= _returnvalue OtherActor)
      (`AISense_Hearing.ReportNoiseEvent` _returnvalue_2 1.0 _returnvalue)
      (`GameplayStatics.PlaySoundAtLocation` "/Game/Audio/Assets/SelfStudy/A_MetalClang_Cue.A_MetalClang_Cue" _returnvalue_2 (struct) 1.0 1.0 0.0 null null null null))))

(fn `UserConstructionScript`)