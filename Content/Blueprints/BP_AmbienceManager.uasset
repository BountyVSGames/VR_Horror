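; BP_AmbienceManager is an actor that drives the game's underwater ambient audio.
; On BeginPlay a timeline fades the volume multiplier of the underwater ambience cue.
; Tick counts down a timer, then picks a random BP_AmbienceEvent in the level, calls PlaySoundEvent on it and resets the timer to a random delay between configurable minimum and maximum values.
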(event `self.ReceiveBeginPlay`
  (bind (_direction _volumemultiplier) (`Timeline|SoundFadeTimeline` :!via `PlayFromStart`)
    (:`Update`
      (`AudioComponent.SetVolumeMultiplier` (`self.A_UnderwaterAmbience_Cue`) _volumemultiplier))))

(event `self.ReceiveTick`
  (params (DeltaSeconds :type "Float (single-precision)"))
  (bind _output_get (set `self.Timer` (- (`self.Timer`) DeltaSeconds)))
  (if (<= _output_get 0.0)
    (bind _outactors (`GameplayStatics.GetAllActorsOfClass` "/Game/Blueprints/BP_AmbienceEvent.BP_AmbienceEvent_C"))
    (`/Game/Blueprints/BP_AmbienceEvent.PlaySoundEvent` (`KismetArrayLibrary.Array_Random` _outactors))
    (set `self.Timer` (`KismetMathLibrary.RandomFloatInRange` (`self.MinSoundDelay`) (`self.MaxSoundDelay`)))))

(fn `UserConstructionScript`)