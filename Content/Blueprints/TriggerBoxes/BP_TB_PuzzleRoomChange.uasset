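; Trigger box that starts the puzzle room change event when the light switch is pressed after the player enters it.
; On player overlap, it finds BP_LightSwitch and starts a looping timer that polls the switch's VR button.
; Once the button is in use, it calls StartEvent on BP_SE_PuzzleRoomChange and destroys itself.
; No end-overlap check exists, so polling continues after the player leaves the box.
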(event `self.ReceiveActorBeginOverlap`
  (params (OtherActor :type "Actor Object Reference"))
  ;[0.6978 0.6178 1] Checks if the player is hitting the light switch while overlapping, if so starts the event and destroys itself
  (cast `/Game/Blueprints/Player/BP_Player` OtherActor)
  (bind _returnvalue (`GameplayStatics.GetActorOfClass` "/Game/Blueprints/Interactions/BP_LightSwitch.BP_LightSwitch_C"))
  (`KismetSystemLibrary.K2_SetTimerDelegate` (delegate `Check`) 0.1 true))

(event `Check`
  ;[0.6978 0.6178 1] Checks if the player is hitting the light switch while overlapping, if so starts the event and destroys itself
  (if (`VRButtonComponent.IsButtonInUse` (`/Game/Blueprints/Interactions/BP_LightSwitch.VRButton` (stale `self.ReceiveActorBeginOverlap` _returnvalue)))
    (bind _returnvalue (`GameplayStatics.GetActorOfClass` "/Game/Blueprints/ScriptedEvents/BP_SE_PuzzleRoomChange.BP_SE_PuzzleRoomChange_C"))
    (`/Engine/EditorBlueprintResources/StandardMacros.IsValid` _returnvalue
      (:`Is Valid`
        (`ScriptedEvent.StartEvent` _returnvalue true)
        (`self.K2_DestroyActor`)))))

(fn `UserConstructionScript`)