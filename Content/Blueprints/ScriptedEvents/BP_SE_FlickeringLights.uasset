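; Scripted event that flickers the submarine's lights for five seconds when it starts.
; FlickerLights re-triggers itself after short random delays, toggling the shared BP_LightDarkManager found on BeginPlay.
; A timer then calls StopFlickering, which restores light if it is dark, completes the event and destroys the actor, ending the loop.
; The BP_SubmarineLight actors gathered at start are stored but not used here.
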(event `self.ReceiveBeginPlay`
  (bind _returnvalue (`GameplayStatics.GetActorOfClass` "/Game/Blueprints/Light-Dark_System/BP_LightDarkManager.BP_LightDarkManager_C"))
  (set `self.LightDarkRef` _returnvalue))

(event `self.OnEventStarted`
  (bind _outactors (`GameplayStatics.GetAllActorsOfClass` "/Game/Blueprints/Light-Dark_System/BP_SubmarineLight.BP_SubmarineLight_C"))
  (set `self.Lights` _outactors)
  (`KismetSystemLibrary.K2_SetTimer` null "StopFlickering" 5.0)
  (`self.FlickerLights`))

(event `FlickerLights`
  (`/Game/Blueprints/Light-Dark_System/BP_LightDarkManager.ToggleLights` (`self.LightDarkRef`))
  (`KismetSystemLibrary.Delay` (`KismetMathLibrary.RandomFloatInRange` 0.1 0.35))
  (`self.FlickerLights`))

(fn `StopFlickering`
  (bind _lightdarkref (`self.LightDarkRef`))
  (if (not (`/Game/Blueprints/Light-Dark_System/BP_LightDarkManager.IsLight` _lightdarkref))
    (`/Game/Blueprints/Light-Dark_System/BP_LightDarkManager.ToggleLights` _lightdarkref))
  (`self.CompleteEvent` true)
  (`self.K2_DestroyActor`))

(fn `UserConstructionScript`)