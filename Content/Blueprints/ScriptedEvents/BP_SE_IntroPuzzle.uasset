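; Scripted event for the intro puzzle that stages a scare-like scene change, then destroys itself.
; On start, it flickers lights through BP_LightDarkManager at random intervals, turns the lock lamp red and moves it, hides letter text and moves tagged boxes.
; Targets are found by actor tags, with the box destination cached at BeginPlay.
; A three-second timer leaves the world dark and completes the event; OpenLockerDoor is defined but not called here.
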(event `self.ReceiveBeginPlay`
  ;[0.9667 0.7292 1] Get references to light / dark system and light switch(es)
  (bind _returnvalue (`GameplayStatics.GetActorOfClass` "/Game/Blueprints/Light-Dark_System/BP_LightDarkManager.BP_LightDarkManager_C"))
  (set `self.LightDarkRef` _returnvalue)
  (bind _outactors (`GameplayStatics.GetAllActorsOfClass` "/Game/Blueprints/Interactions/BP_LightSwitch.BP_LightSwitch_C"))
  (for _array_element _outactors
    (set `self.Array Element` _array_element)
    (bind _outactors_2 (`GameplayStatics.GetAllActorsOfClassWithTag` "/Script/Engine.TargetPoint" "Box1Move"))
    (for _array_element_2 _outactors_2
      (set `self.BoxesLocation` (`self.K2_GetActorLocation` _array_element_2)))))

(event `self.OnEventStarted`
  ;[0.5729 0.9097 1] Rotate doors, move lamp and flicker lights
  (`|ExecutionSequence`
    (:`then_0`
      (bind _outactors (`GameplayStatics.GetAllActorsOfClass` "/Game/Blueprints/Light-Dark_System/BP_SubmarineLight.BP_SubmarineLight_C"))
      (set `self.Lights` _outactors)
      (`KismetSystemLibrary.K2_SetTimer` null "StopFlickering" 3.0)
      (`self.FlickerLights`))
    (:`then_2`
      (`self.Move Lamp and Change Light Color`))
    (:`then_3`
      (`self.RemoveRevealedLetter`))
    (:`then_4`
      (bind _outactors_2 (`GameplayStatics.GetAllActorsOfClassWithTag` "/Script/Engine.StaticMeshActor" "Box1"))
      (for _array_element _outactors_2
        (`self.K2_SetActorLocation` _array_element (`self.BoxesLocation`) false false)))))

(event `FlickerLights`
  ;[0.5705 0.6356 1] Flicker lights
  (`/Game/Blueprints/Light-Dark_System/BP_LightDarkManager.ToggleLights` (`self.LightDarkRef`))
  (`KismetSystemLibrary.Delay` (`KismetMathLibrary.RandomFloatInRange` 0.1 0.25))
  (`self.FlickerLights`))

(fn `Move Lamp and Change Light Color`
  (bind _returnvalue (`GameplayStatics.GetActorOfClass` "/Game/Blueprints/Interactions/KeyLockSystem/BP_LockLamp.BP_LockLamp_C"))
  (bind _pointlight (`/Game/Blueprints/Interactions/KeyLockSystem/BP_LockLamp.PointLight` _returnvalue))
  (`LightComponent.SetIntensity` _pointlight 50.0)
  (`LightComponent.SetLightColor` _pointlight (struct :`R` 0.864583 :`A` 1.0) true)
  (bind _outactors (`GameplayStatics.GetAllActorsOfClassWithTag` "/Script/Engine.TargetPoint" "Lamp"))
  (for _array_element _outactors
    (bind (_returnvalue_location _returnvalue_rotation _returnvalue_scale) (`KismetMathLibrary.BreakTransform` (`self.GetTransform` _array_element)))
    (`self.K2_SetActorTransform` _returnvalue (`KismetMathLibrary.MakeTransform` _returnvalue_location _returnvalue_rotation _returnvalue_scale) false false)))

(fn `OpenLockerDoor`
  (bind _outactors (`GameplayStatics.GetAllActorsOfClass` "/Game/Blueprints/Interactions/BP_Door.BP_Door_C"))
  (for _array_element _outactors
    (if (`self.ActorHasTag` _array_element "LockerDoor02")
      (bind _vrlever (`/Game/Blueprints/Interactions/BP_Door.VRLever` _array_element))
      (`VRLeverComponent.SetLeverAngle` _vrlever 150.0 (0.0 0.0 0.0) true)
      (set `VRLeverComponent.bIsLocked` false _vrlever))))

(fn `RemoveRevealedLetter`
  (bind _outactors (`GameplayStatics.GetAllActorsOfClass` "/Script/Engine.TextRenderActor"))
  (for _array_element _outactors
    (if (`self.ActorHasTag` _array_element "Letter")
      (`SceneComponent.SetVisibility` (`TextRenderActor.TextRender` _array_element) false false))))

(fn `StopFlickering`
  (bind _lightdarkref (`self.LightDarkRef`))
  (if (`/Game/Blueprints/Light-Dark_System/BP_LightDarkManager.IsLight` _lightdarkref)
    (`/Game/Blueprints/Light-Dark_System/BP_LightDarkManager.ToggleLights` _lightdarkref))
  (`self.CompleteEvent` true)
  (`self.K2_DestroyActor`))

(fn `UserConstructionScript`)