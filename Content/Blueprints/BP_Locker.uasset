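; BP_Locker is a VR locker that the player can teleport into and back out of.
; Opening the VRLever door far enough, or being inside, reveals DoorTrigger, whose overlaps with controller trigger components arm the left or right trigger input.
; That input calls Door, which saves a head-based return position, teleports the player inside, then zeroes and locks the lever.
; Calling it again returns the player and unlocks the lever.
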(event `self.ReceiveBeginPlay`
  (`SceneComponent.SetVisibility` (`self.DoorTrigger`) false false)
  (`PrimitiveComponent.SetCollisionResponseToAllChannels` (`self.DoorTrigger`) "ECR_Ignore")
  (bind _returnvalue (`GameplayStatics.GetActorOfClass` "/Game/Blueprints/Player/BP_Player.BP_Player_C"))
  (set `self.Player` _returnvalue))

(event `self.ReceiveTick`
  (params (DeltaSeconds :type "Float (single-precision)"))
  (if (> (`VRLeverComponent.CurrentLeverAngle` (`self.VRLever`)) 25.0)
    (`SceneComponent.SetVisibility` (`self.DoorTrigger`) true false :!label _label)
    (`PrimitiveComponent.SetCollisionResponseToAllChannels` (`self.DoorTrigger`) "ECR_Overlap")
    (elif (`self.InsideLocker`)
      (goto _label)
      (else
        (`SceneComponent.SetVisibility` (`self.DoorTrigger`) false false)
        (`PrimitiveComponent.SetCollisionResponseToAllChannels` (`self.DoorTrigger`) "ECR_Ignore")))))

(event `InputTriggerLeft`
  (if (`self.LeftTriggerable`)
    (`self.Door`)))

(event `InputTriggerRight`
  (if (`self.RightTriggerable`)
    (`self.Door`)))

(event `self.DoorTrigger.OnComponentBeginOverlap`
  (params (OverlappedComponent :type "PrimitiveComponent Object Reference") (OtherActor :type "Actor Object Reference") (OtherComp :type "PrimitiveComponent Object Reference") (OtherBodyIndex :type Integer) (bFromSweep :type Boolean) (SweepResult :type "HitResult Structure (by ref)"))
  (bind _returnvalue (`KismetSystemLibrary.GetDisplayName` OtherComp))
  (`KismetSystemLibrary.PrintString` _returnvalue)
  (if (and (`KismetStringLibrary.Contains` _returnvalue "Right Trigger") (`SceneComponent.bVisible` (`self.DoorTrigger`)))
    (set `self.RightTriggerable` true)
    (elif (`KismetStringLibrary.Contains` _returnvalue "Left Trigger")
      (set `self.LeftTriggerable` true))))

(event `self.DoorTrigger.OnComponentEndOverlap`
  (params (OverlappedComponent :type "PrimitiveComponent Object Reference") (OtherActor :type "Actor Object Reference") (OtherComp :type "PrimitiveComponent Object Reference") (OtherBodyIndex :type Integer))
  (bind _returnvalue (`KismetSystemLibrary.GetDisplayName` OtherComp))
  (bind _bvisible (`SceneComponent.bVisible` (`self.DoorTrigger`)))
  (if (and (`KismetStringLibrary.Contains` _returnvalue "Right Trigger") _bvisible)
    (set `self.RightTriggerable` false)
    (elif (and _bvisible (`KismetStringLibrary.Contains` _returnvalue "Left Trigger"))
      (set `self.LeftTriggerable` false))))

(fn `Door`
  (bind _player (`self.Player`))
  (bind _vrlever (`self.VRLever`))
  (bind (_returnvalue_x _returnvalue_y _returnvalue_z) (`KismetMathLibrary.BreakVector` (`self.K2_GetActorLocation` _player)))
  (bind (_returnvalue_x_2 _returnvalue_y_2) (`KismetMathLibrary.BreakVector` (`SceneComponent.K2_GetComponentLocation` (`self.TeleportLocation`))))
  (bind (_returnvalue_x_3 _returnvalue_y_3 _returnvalue_z_2) (`KismetMathLibrary.BreakVector` (`VRBaseCharacter.K2_GetVRHeadLocation` _player)))
  (if (`self.InsideLocker`)
    (`VRBaseCharacter.SetActorLocationAndRotationVR` :`self` (`self.Player`) :`NewLoc` (`self.OldLocation`) :`bRotateAroundCapsule` false)
    (set `self.LeftTriggerable` false)
    (set `self.InsideLocker` false)
    (set `VRLeverComponent.LeverReturnTypeWhenReleased` "RetainMomentum" (`self.VRLever`))
    (set `VRLeverComponent.bDenyGripping` false (`self.VRLever`))
    (else
      (set `self.OldLocation` (`KismetMathLibrary.MakeVector` _returnvalue_x_3 _returnvalue_y_3 (- _returnvalue_z_2 200.0)))
      (`VRBaseCharacter.SetActorLocationAndRotationVR` _player (`KismetMathLibrary.MakeVector` _returnvalue_x_2 _returnvalue_y_2 _returnvalue_z) (struct :`Yaw` 180.0) true true false false)
      (set `self.LeftTriggerable` false)
      (set `VRLeverComponent.LeverReturnTypeWhenReleased` "ReturnToZero" _vrlever)
      (`VRLeverComponent.SetLeverAngle` _vrlever 0.0 (0.0 0.0 0.0) true)
      (set `self.InsideLocker` true)
      (set `VRLeverComponent.bDenyGripping` true (`self.VRLever`)))))

(fn `UserConstructionScript`)