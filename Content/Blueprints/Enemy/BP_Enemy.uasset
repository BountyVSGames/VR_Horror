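; BP_Enemy is an AI enemy that hunts the player and kills on overlap with their head collision.
; AI perception drives a state enum written to the Blackboard: hearing triggers investigation, while trace-checked sight escalates on a timer.
; BP_LightDarkManager's dispatcher toggles it: lights on disable sight and hide the mesh but keep its shadow, lights off restore both.
; Timed footsteps and a spotted cue provide audio feedback.
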(event `Try Play Grunt`
  ;[1 0.07812 0.6494] When enemy is not moving, play grunts
)

(event `Set Audio Timers`
  ;[1 0.07812 0.6494] Audio timer setup
  (`|ExecutionSequence`
    (:`then_0`
      ;[1 0.07812 0.6494] When enemy is not moving, play grunts
      (`KismetSystemLibrary.K2_SetTimerDelegate` (delegate `Try Play Grunt`) 4.0 true))
    (:`then_1`
      ;[1 0.07812 0.6494] When enemy is moving, play footsteps.
      (`KismetSystemLibrary.K2_SetTimerDelegate` (delegate `Try Play Footstep`) 1.2 true))))

(event `Try Play Footstep`
  ;[1 0.07812 0.6494] When enemy is moving, play footsteps.
  (if (> (`KismetMathLibrary.VSize` (`MovementComponent.Velocity` (`self.CharacterMovement`))) 0.01)
    (`AudioComponent.Play` (`self.A_PLACEHOLDER_EnemyStep_Cue`) 0.0)))

(event `self.ReceiveBeginPlay`
  (bind _aiperception (`self.AIPerception`))
  (bind _asbp_player (cast `/Game/Blueprints/Player/BP_Player` (`GameplayStatics.GetPlayerCharacter` 0)))
  (set `self.PlayerHead` (`/Game/Blueprints/Player/BP_Player.HeadCollision` _asbp_player))
  (bind _returnvalue (`GameplayStatics.GetActorOfClass` "/Game/Blueprints/Light-Dark_System/BP_LightDarkManager.BP_LightDarkManager_C"))
  (set `/Game/Blueprints/Light-Dark_System/BP_LightDarkManager.IsLight` false _returnvalue)
  (if (`/Game/Blueprints/Light-Dark_System/BP_LightDarkManager.IsLight` _returnvalue)
    (`AIPerceptionComponent.SetSenseEnabled` _aiperception "/Script/VRExpansionPlugin.AISense_Sight_VR" false)
    (`AIPerceptionComponent.SetSenseEnabled` _aiperception "/Script/AIModule.AISense_Sight" false)
    (`SceneComponent.SetVisibility` (`self.Mesh`) false false)
    (set `self.IsInLight` false)
    (`PrimitiveComponent.SetCastHiddenShadow` (`self.Mesh`) true))
  (add `/Game/Blueprints/Light-Dark_System/BP_LightDarkManager.ToggleLightsDispatcher` _returnvalue (delegate `OnLightsToggled`))
  (`self.Set Audio Timers`))

(event `OnLightsToggled`
  (params (IsLight :type Boolean))
  (bind _aiperception (`self.AIPerception`))
  (bind _aiperception_2 (`self.AIPerception`))
  (if IsLight
    (`AIPerceptionComponent.SetSenseEnabled` _aiperception_2 "/Script/VRExpansionPlugin.AISense_Sight_VR" false)
    (`AIPerceptionComponent.SetSenseEnabled` _aiperception_2 "/Script/AIModule.AISense_Sight" false)
    (`SceneComponent.SetVisibility` (`self.Mesh`) false false)
    (set `self.IsInLight` false)
    (`PrimitiveComponent.SetCastHiddenShadow` (`self.Mesh`) true)
    (else
      (`AIPerceptionComponent.SetSenseEnabled` _aiperception "/Script/VRExpansionPlugin.AISense_Sight_VR" true)
      (`AIPerceptionComponent.SetSenseEnabled` _aiperception "/Script/AIModule.AISense_Sight" true)
      (`SceneComponent.SetVisibility` (`self.Mesh`) true false)
      (set `self.IsInLight` true)
      (`self.Change state` "NewEnumerator0"))))

(event `self.ReceiveTick`
  (params (DeltaSeconds :type "Float (single-precision)"))
  (`|ExecutionSequence`
    (:`then_0`
      ;[1 0.07812 0.6494] Play Alerted sound effect when state changes to investigate.
      (if (not (`|EnumEquality` (`self.EnemyState`) (`self.Old Enemy State`)))
        (`|ExecutionSequence`
          (:`then_0`
            (if (`|EnumEquality` (`self.EnemyState`) "NewEnumerator1")
              (`AudioComponent.Play` (`self.A_PLACEHOLDER_EnemySpotted_Cue`) 0.0)))
          (:`then_1`
            (`KismetSystemLibrary.DelayUntilNextTick`)
            (set `self.Old Enemy State` (`self.EnemyState`))))))
    (:`then_1`
      (if (`self.PlayerInSight`)
        (bind _output_get (set `self.PlayerInSightTimer` (+ (`self.PlayerInSightTimer`) 0.1)))
        (if (> _output_get 10.0)
          (`self.Change state` "NewEnumerator2")
          (else
            (`self.Change state` "NewEnumerator3")))))))

(event `self.AIPerception.OnTargetPerceptionUpdated`
  (params (Actor :type "Actor Object Reference") (Stimulus :type "AIStimulus Structure"))
  (bind (_age _expirationage _strength _stimuluslocation _receiverlocation _tag _bsuccessfullysensed) (break `AIStimulus` Stimulus))
  (bind _returnvalue (`AIPerceptionSystem.GetSenseClassForStimulus` Stimulus))
  (if (== _returnvalue "/Script/AIModule.AISense_Hearing")
    (set `self.InvestigateLocation` (`.StimulusLocation` (break `AIStimulus` Stimulus)))
    (`self.Change state` "NewEnumerator1")
    (elif (== Actor (`GameplayStatics.GetPlayerCharacter` 0))
      (bind _asbp_player (cast `/Game/Blueprints/Player/BP_Player` (`GameplayStatics.GetPlayerCharacter` 0)))
      (bind _returnvalue_2 (`SceneComponent.K2_GetComponentLocation` (`/Game/Blueprints/Player/BP_Player.HeadCollision` _asbp_player)))
      (bind _outhit (`KismetSystemLibrary.SphereTraceSingle` _receiverlocation (+ (* (`KismetMathLibrary.Normal` (`KismetMathLibrary.GetDirectionUnitVector` _receiverlocation _returnvalue_2)) 10) _returnvalue_2) 30.0 "TraceTypeQuery1"))
      (if (== (`.HitActor` (`GameplayStatics.BreakHitResult` _outhit)) (`GameplayStatics.GetPlayerCharacter` 0))
        (set `self.InvestigateLocation` _stimuluslocation)
        (if _bsuccessfullysensed
          (set `self.PlayerInSight` true)
          (`self.Change state` "NewEnumerator3")
          (else
            (set `self.PlayerInSight` false :!label _label)
            (set `self.PlayerInSightTimer` 0.0)
            (`self.Change state` "NewEnumerator1")))
        (else
          (set `self.InvestigateLocation` _stimuluslocation)
          (`KismetSystemLibrary.RetriggerableDelay` (`self.ChargeDuration`))
          (goto _label))))))

(event `self.OverlapCollsion.OnComponentBeginOverlap`
  (params (OverlappedComponent :type "PrimitiveComponent Object Reference") (OtherActor :type "Actor Object Reference") (OtherComp :type "PrimitiveComponent Object Reference") (OtherBodyIndex :type Integer) (bFromSweep :type Boolean) (SweepResult :type "HitResult Structure (by ref)"))
  (bind _asbp_player (cast `/Game/Blueprints/Player/BP_Player` OtherActor))
  (if (== OtherComp (`/Game/Blueprints/Player/BP_Player.HeadCollision` _asbp_player))
    (`/Game/Blueprints/Player/BP_Player.OnPlayerDeath` _asbp_player)))

(fn `Change state`
  (params (StateChange :type "/Game/Blueprints/Enemy/E_EnemyState Enum" :default "NewEnumerator0"))
  (locals (State :type Name :default "State"))
  (bind _output_get (set `self.EnemyState` StateChange))
  (`BlackboardComponent.SetValueAsEnum` (`AIBlueprintHelperLibrary.GetBlackboard` null) (`local.State`) _output_get))

(fn `ChasePlayer`)

(fn `Investigate`
  (params (NewParam :type "/Game/Blueprints/Enemy/E_EnemyState Enum" :default "NewEnumerator0"))
  (locals (State :type Name :default "State"))
  (bind _output_get (set `self.EnemyState` "NewEnumerator1"))
  (`BlackboardComponent.SetValueAsEnum` (`AIBlueprintHelperLibrary.GetBlackboard` null) (`local.State`) _output_get))

(fn `SetSpeed`
  (params (Speed :type "Float (double-precision)"))
  (set `CharacterMovementComponent.MaxWalkSpeed` Speed (`self.CharacterMovement`)))

(fn `UserConstructionScript`
  (`SceneComponent.K2_AttachToComponent` (`self.NS_Breathing`) (`self.Mesh`) "head" "KeepRelative" "KeepRelative" "KeepRelative" true))