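; Submarine spotlight actor in the Light-Dark system that responds to light toggle events.
; On BeginPlay it hides the light mesh, caches the spotlight's intensity and, if set to start off, plays a timeline that lerps intensity toward zero.
; Toggle events switch spotlight visibility directly, while a branch that would play or reverse the fade on toggle is left disconnected.
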(event `self.ReceiveBeginPlay`
  (`parent.ReceiveBeginPlay`)
  (`SceneComponent.SetVisibility` (`self.LightMesh`) false false)
  (set `self.DefaultIntensity` (`LightComponentBase.Intensity` (`self.SpotLight`)))
  (if (`self.StartOff`)
    (bind (_direction _newtrack_0) (`Timeline|LightsFade`)
      (:`Update`
        (`LightComponent.SetIntensity` (`self.SpotLight`) (`KismetMathLibrary.Lerp` (`self.DefaultIntensity`) 0.0 _newtrack_0))))))

(event `self.OnLightsToggled`
  (params (IsLight :type Boolean))
  (`SceneComponent.SetVisibility` (`self.SpotLight`) IsLight false))

(fn `UserConstructionScript`
  (`parent.UserConstructionScript`))