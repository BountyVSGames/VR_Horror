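; BP_LightDarkParent is a base actor for objects that respond to the game's light and dark state.
; On BeginPlay it binds OnLightsToggled, an empty event here, to the toggle dispatcher on BP_LightDarkManager.
; Overlap begin and end with a BP_Flashlight set InFlashlight and re-fire OnLightsToggled with the IsLight state, so flashlight exposure and global toggles share one handler.
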(event `self.ReceiveBeginPlay`
  ;[1 1 1] Bind Event
  (bind _returnvalue (`GameplayStatics.GetActorOfClass` "/Game/Blueprints/Light-Dark_System/BP_LightDarkManager.BP_LightDarkManager_C"))
  (add `/Game/Blueprints/Light-Dark_System/BP_LightDarkManager.ToggleLightsDispatcher` _returnvalue (delegate `OnLightsToggled`)))

(event `OnLightsToggled`
  (params (IsLight :type Boolean))
  ;[1 1 1] Bind Event
)

(event `self.ReceiveActorBeginOverlap`
  (params (OtherActor :type "Actor Object Reference"))
  ;[1 1 1] Flashlight detection
  (cast `/Game/Blueprints/Flashlight/BP_Flashlight` OtherActor)
  (`GameplayStatics.GetActorOfClass` "/Game/Blueprints/Light-Dark_System/BP_LightDarkManager.BP_LightDarkManager_C")
  (set `self.InFlashlight` true)
  (`self.OnLightsToggled` (stale `OnLightsToggled` IsLight)))

(event `self.ReceiveActorEndOverlap`
  (params (OtherActor :type "Actor Object Reference"))
  ;[1 1 1] Flashlight detection
  (cast `/Game/Blueprints/Flashlight/BP_Flashlight` OtherActor)
  (`GameplayStatics.GetActorOfClass` "/Game/Blueprints/Light-Dark_System/BP_LightDarkManager.BP_LightDarkManager_C")
  (set `self.InFlashlight` false)
  (`self.OnLightsToggled` (stale `OnLightsToggled` IsLight)))

(fn `UserConstructionScript`)