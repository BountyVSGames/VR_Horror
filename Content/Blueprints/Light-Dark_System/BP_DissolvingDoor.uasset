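; Door in the light-dark system that dissolves or reappears with the lighting, with VisibleInLight choosing which state shows it.
; BeginPlay creates a dynamic M_Dissolver material and starts doors not visible in light dissolving.
; OnLightsToggled plays or reverses the dissolve timeline, treating flashlight exposure as light.
; The timeline drives the Dissolve parameter and, when finished, enables collision only if the door is fully solid.
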(event `self.ReceiveBeginPlay`
  (bind _doorcollision (`self.DoorCollision`))
  ;[1 1 1] Ensure preset boolean is processed
  (`parent.ReceiveBeginPlay`)
  (bind _returnvalue (`PrimitiveComponent.CreateDynamicMaterialInstance` (`self.Door`) 0 "/Game/Materials/M_Dissolver.M_Dissolver" "None"))
  (set `self.DissolveMaterial` _returnvalue)
  (if (not (`self.VisibleInLight`))
    (bind (_direction _dissolve) (`Timeline|DissolveTimeline` :!label _label)
      (:`Update`
        ;[1 1 1] Set material dissolve percentage based on timeline
        (`MaterialInstanceDynamic.SetScalarParameterValue` (`self.DissolveMaterial`) "Dissolve" _dissolve))
      (:`Finished`
        ;[1 1 1] Set collision based on current visual state
        (if (== _dissolve 0.0)
          (`PrimitiveComponent.SetCollisionEnabled` _doorcollision "QueryAndPhysics")
          (else
            (`PrimitiveComponent.SetCollisionEnabled` _doorcollision "NoCollision")))))))

(event `self.OnLightsToggled`
  (params (IsLight :type Boolean))
  (if (`self.VisibleInLight`)
    (if (or IsLight (`self.InFlashlight`))
      (goto _label :!via `Reverse`)
      (else
        (goto _label)))
    (elif (or IsLight (`self.InFlashlight`))
      (goto _label)
      (else
        (goto _label :!via `Reverse`)))))

(fn `UserConstructionScript`
  (`parent.UserConstructionScript`))