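; Light/Dark system actor that moves along a target spline and transforms as the lights toggle.
; A SplineMovement timeline starts on BeginPlay, then reverses on light and plays forward on dark.
; Its alpha drives position along the spline and, with a valid spline, lerps mesh scale and actor rotation from initial to target values where they differ.
; Tick prints the actor's location for debugging.
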(event `self.ReceiveBeginPlay`
  (bind _baserotation (`self.BaseRotation`))
  (bind _targetrotation (`self.TargetRotation`))
  (bind _targetscale (`self.TargetScale`))
  (bind _basescale (`self.BaseScale`))
  (bind _spline (`/Game/Blueprints/Light-Dark_System/BP_TargetSpline.Spline` (`self.TargetSpline`)))
  (`parent.ReceiveBeginPlay`)
  (set `self.BaseScale` (`self.GetActorScale3D`))
  (set `self.BaseRotation` (`self.K2_GetActorRotation`))
  (bind (_direction _alpha) (`Timeline|SplineMovement` :!label _label)
    (:`Update`
      (set `self.Alpha` _alpha)
      (`/Engine/EditorBlueprintResources/StandardMacros.IsValid` (`self.TargetSpline`)
        (:`Is Valid`
          (`self.K2_SetActorLocation` (`SplineComponent.GetLocationAtDistanceAlongSpline` _spline (`KismetMathLibrary.Lerp` 0.0 (`SplineComponent.GetSplineLength` _spline) (`self.Alpha`)) "World"))
          (`|ExecutionSequence`
            (:`then_0`
              (if (!= _basescale _targetscale)
                (`SceneComponent.SetWorldScale3D` (`self.MeshRef`) (`KismetMathLibrary.VLerp` _basescale _targetscale (`self.Alpha`)))))
            (:`then_1`
              (if (!= _baserotation _targetrotation)
                (`self.K2_SetActorRotation` (`KismetMathLibrary.RLerp` _baserotation _targetrotation (`self.Alpha`)))))))))))

(event `self.ReceiveTick`
  (params (DeltaSeconds :type "Float (single-precision)"))
  (`KismetSystemLibrary.PrintString` (`KismetStringLibrary.Conv_VectorToString` (`self.K2_GetActorLocation`))))

(event `self.OnLightsToggled`
  (params (IsLight :type Boolean))
  (if IsLight
    (goto _label :!via `Reverse`)
    (else
      (goto _label))))

(fn `UserConstructionScript`
  (`parent.UserConstructionScript`))